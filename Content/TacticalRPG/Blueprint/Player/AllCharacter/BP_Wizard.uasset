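; BP_Wizard is the Wizard character in the tactical RPG, driving its Sevarog Animation Blueprint through idle, walk and chosen-emote states.
; It caches the AnimBP on BeginPlay, then the Idle, Walk and OnChosen events set its pose index, with OnChosen picking one of two emotes at random.
; While emoting, Tick accumulates play time and passes it to the AnimBP.
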(event `self.ReceiveBeginPlay`
  ;[1 1 1] Begin Play
  (set `self.As ABP Sevarog` (cast `/Game/TacticalRPG/Blueprint/Animation/ABP_Sevarog` (`SkeletalMeshComponent.GetAnimInstance` (`self.Mesh`)) :!pure true)))

(event `self.ReceiveTick`
  (params (DeltaSeconds :type "Float (single-precision)"))
  ;[1 1 1] Tick
  (if (`self.isEmoting`)
    (bind _output_get (set `self.emotePlayTime` (+ (`self.emotePlayTime`) DeltaSeconds)))
    (set `/Game/TacticalRPG/Blueprint/Animation/ABP_Sevarog.playTime` _output_get (`self.As ABP Sevarog`))))

(event `self.OnChosen`
  (set `self.emotePlayTime` 0.0)
  (set `/Game/TacticalRPG/Blueprint/Animation/ABP_Sevarog.playTime` 0.0 (`self.As ABP Sevarog`))
  (`self.StopAnimMontage` null)
  (set `/Game/TacticalRPG/Blueprint/Animation/ABP_Sevarog.poses` (`KismetMathLibrary.RandomIntegerInRange` 2 3) (`self.As ABP Sevarog`))
  (set `self.isEmoting` true))

(event `self.Walk`
  (`self.StopAnimMontage` null)
  (set `/Game/TacticalRPG/Blueprint/Animation/ABP_Sevarog.poses` 1 (`self.As ABP Sevarog`))
  (set `self.isEmoting` false))

(event `self.Idle`
  (set `/Game/TacticalRPG/Blueprint/Animation/ABP_Sevarog.poses` 0 (`self.As ABP Sevarog`))
  (set `self.isEmoting` false))

(fn `UserConstructionScript`
  (`parent.UserConstructionScript`))